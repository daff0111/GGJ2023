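; BP_Boss is a boss pawn that pursues the player, kills on overlap and destroys static mesh actors it touches.
; BeginPlay caches the player pawn and health bar widget, then starts a single AI move toward the player.
; Tick rubber-bands the boss along Y with a swept move so it trails at most 1500 units behind.
; Overlapping the player disables their input and ragdolls the mesh; the health bar tint logic never runs.
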(event `self.ReceiveBeginPlay`
  (set `self.HeroesActor` (`GameplayStatics.GetPlayerPawn` 0))
  (bind _asbp_health_bar_2 (cast `/Game/Widgets/BP_HealthBar2` (`WidgetComponent.GetUserWidgetObject` (`self.Widget`))))
  (`|AIMoveTo` self (0.0 0.0 0.0) (`self.HeroesActor`) 0.0))

(event `self.ReceiveTick`
  (params (DeltaSeconds :type "Float (single-precision)"))
  (bind (_returnvalue_x _returnvalue_y _returnvalue_z) (`KismetMathLibrary.BreakVector` (`self.K2_GetActorLocation`)))
  (bind (_returnvalue_x_2 _returnvalue_y_2) (`KismetMathLibrary.BreakVector` (`self.K2_GetActorLocation` (`self.HeroesActor`))))
  (bind _returnvalue (- _returnvalue_y_2 1500.0))
  (if (< _returnvalue_y _returnvalue)
    (`self.K2_SetActorLocation` (`KismetMathLibrary.MakeVector` _returnvalue_x _returnvalue _returnvalue_z) true)))

(event `self.ReceiveActorBeginOverlap`
  (params (OtherActor :type "Actor Object Reference"))
  (bind _returnvalue (`GameplayStatics.GetObjectClass` OtherActor))
  ;[1 1 1] Kill
  (if (== _returnvalue "/Game/ThirdPerson/Blueprints/BP_ThirdPersonCharacter.BP_ThirdPersonCharacter_C")
    (bind _asbp_third_person_character (cast `/Game/ThirdPerson/Blueprints/BP_ThirdPersonCharacter` OtherActor))
    (bind _asplayer_controller (cast `PlayerController` (`self.GetController` _asbp_third_person_character)))
    (`self.DisableInput` _asbp_third_person_character _asplayer_controller)
    (`PrimitiveComponent.SetSimulatePhysics` (`Character.Mesh` _asbp_third_person_character) true)
    (elif (== _returnvalue "/Script/Engine.StaticMeshActor")
      (`self.K2_DestroyActor` OtherActor))))

(fn `UserConstructionScript`)