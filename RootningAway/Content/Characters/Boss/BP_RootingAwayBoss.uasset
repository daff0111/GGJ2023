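; BP_RootingAwayBoss is a pursuing boss that advances along +Y behind the player and destroys any actor it overlaps.
; On BeginPlay it caches the player pawn, prints a debug message and starts an AI move to a distant point along +Y.
; Each Tick it snaps forward with a swept move whenever it trails the player by more than a fixed Y distance, capping the player's lead.
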(event `self.ReceiveBeginPlay`
  (bind (_returnvalue_x _returnvalue_y _returnvalue_z) (`KismetMathLibrary.BreakVector` (`self.K2_GetActorLocation`)))
  (set `self.HerosActor` (`GameplayStatics.GetPlayerPawn` 0))
  (`KismetSystemLibrary.PrintString` "set successful" true true (struct :`G` 0.66 :`B` 1.0 :`A` 1.0) 10.0)
  (`|AIMoveTo` self (`KismetMathLibrary.MakeVector` _returnvalue_x (+ _returnvalue_y 10000.0) _returnvalue_z) null 0.0))

(event `self.ReceiveActorBeginOverlap`
  (params (OtherActor :type "Actor Object Reference"))
  (`self.K2_DestroyActor` OtherActor))

(event `self.ReceiveTick`
  (params (DeltaSeconds :type "Float (single-precision)"))
  (bind (_returnvalue_x _returnvalue_y _returnvalue_z) (`KismetMathLibrary.BreakVector` (`self.K2_GetActorLocation`)))
  (bind (_returnvalue_x_2 _returnvalue_y_2) (`KismetMathLibrary.BreakVector` (`self.K2_GetActorLocation` (`self.HerosActor`))))
  (bind _returnvalue (- _returnvalue_y_2 1000.0))
  (if (< _returnvalue_y _returnvalue)
    (`self.K2_SetActorLocation` (`KismetMathLibrary.MakeVector` _returnvalue_x _returnvalue _returnvalue_z) true)))

(fn `UserConstructionScript`)