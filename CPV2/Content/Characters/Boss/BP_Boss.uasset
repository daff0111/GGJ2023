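; Boss pawn that chases the player, killing the third-person character on overlap and destroying static mesh actors it touches.
; BeginPlay tints its widget health bar red, starts an AI MoveTo toward the player and runs a looping timer that raises floating movement speed up to a cap.
; Tick rubber-bands the boss along Y so it never falls more than a fixed distance behind the player.
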(event `self.ReceiveBeginPlay`
  (set `self.HeroesActor` (`GameplayStatics.GetPlayerPawn` 0))
  (bind _asbp_health_bar_2 (cast `/Game/Widgets/BP_HealthBar2` (`WidgetComponent.GetUserWidgetObject` (`self.Widget`))))
  (set `/Game/Widgets/BP_HealthBar2.Color` (struct :`R` 1.0 :`A` 1.0) _asbp_health_bar_2)
  (`|AIMoveTo` self (0.0 0.0 0.0) (`self.HeroesActor`) 0.0
    (:`then`
      (`KismetSystemLibrary.K2_SetTimer` null "IncreaseSpeed" 3.0 true))))

(event `self.ReceiveTick`
  (params (DeltaSeconds :type "Float (single-precision)"))
  (bind (_returnvalue_x _returnvalue_y _returnvalue_z) (`KismetMathLibrary.BreakVector` (`self.K2_GetActorLocation`)))
  (bind (_returnvalue_x_2 _returnvalue_y_2) (`KismetMathLibrary.BreakVector` (`self.K2_GetActorLocation` (`self.HeroesActor`))))
  (bind _returnvalue (- _returnvalue_y_2 1500.0))
  (if (< _returnvalue_y _returnvalue)
    (`self.K2_SetActorLocation` (`KismetMathLibrary.MakeVector` _returnvalue_x _returnvalue _returnvalue_z) true)))

(event `self.ReceiveActorBeginOverlap`
  (params (OtherActor :type "Actor Object Reference"))
  (bind _returnvalue (`GameplayStatics.GetObjectClass` OtherActor))
  ;[1 1 1] Kill
  (if (== _returnvalue "/Game/ThirdPerson/Blueprints/BP_ThirdPersonCharacter.BP_ThirdPersonCharacter_C")
    (bind _asbp_third_person_character (cast `/Game/ThirdPerson/Blueprints/BP_ThirdPersonCharacter` OtherActor))
    (`/Game/ThirdPerson/Blueprints/BP_ThirdPersonCharacter.Kill` _asbp_third_person_character)
    (elif (== _returnvalue "/Script/Engine.StaticMeshActor")
      (`self.K2_DestroyActor` OtherActor))))

(fn `IncreaseSpeed`
  (bind _floatingpawnmovement (`self.FloatingPawnMovement`))
  (bind _returnvalue (`MovementComponent.GetMaxSpeed` _floatingpawnmovement))
  (if (<= _returnvalue (`self.MaxSpeed`))
    (set `FloatingPawnMovement.MaxSpeed` (+ _returnvalue (`self.SpeedIncreaseCoeff`)) _floatingpawnmovement)))

(fn `UserConstructionScript`)